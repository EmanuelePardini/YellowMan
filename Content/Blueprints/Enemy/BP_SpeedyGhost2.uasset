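; BP_SpeedyGhost2 is an enemy ghost pawn that wanders by moving toward random nearby navigable points.
; Each Tick, ManageDestination accumulates time and, once the delay elapses, picks a new reachable point within a radius of its current location.
; Tick then issues an AI MoveTo toward the stored destination every frame rather than only when it changes.
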(event EventBeginPlay)

(event Collision|EventActorBeginOverlap
  (params (OtherActor :type Actor%20Object%20Reference)))

(event EventTick
  (params (DeltaSeconds :type Float%20%28single-precision%29))
  (CallFunction|ManageDestination DeltaSeconds)
  (AI|AIMoveTo self (Variables|Default|GetDestinationLoc) 0 5e+01 false))

(fn ConstructionScript)

(fn ManageDestination
  (params (DeltaTime :type Float%20%28double-precision%29))
  (bind _output_get (Variables|Default|SetSetLocTimer (+ DeltaTime (Variables|Default|GetSetLocTimer))))
  (if (>= _output_get (Variables|Default|GetSetLocDelay))
    (Variables|Default|SetSetLocTimer 0.0)
    (Variables|Default|SetDestinationLoc (.RandomLocation (AI|Navigation|GetRandomReachablePointinRadius (Transformation|GetActorLocation) 3.5e+02 0 0)))))